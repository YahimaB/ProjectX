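; Zero-gravity emulator interactable, a child Blueprint that registers itself with the player character while the cursor hovers over it.
; Cursor-over events on AccelCollider cast player 0's character to BP_PlayerCharacter and set its ItemUnderMouse to this actor, then clear it when the cursor leaves.
; A failed cast prints an error, and the construction script only calls the parent's.
; No zero-gravity behavior is implemented in these graphs.
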(event `self.ReceiveBeginPlay`)

(event `self.AccelCollider.OnBeginCursorOver`
  (params (TouchedComponent :type "PrimitiveComponent Object Reference"))
  (bind _asbp_player_character (cast `/Game/FirstProject/Core/Character/BP_PlayerCharacter` (`GameplayStatics.GetPlayerCharacter` 0))
    (:`then`
      (set `PlayerCharacter.itemUnderMouse` self _asbp_player_character))
    (:`CastFailed`
      (`KismetSystemLibrary.PrintString` "Emulator: Cast to Player Controller failed" true true (struct :`R` 1.0 :`A` 1.0) 5.0))))

(event `self.AccelCollider.OnEndCursorOver`
  (params (TouchedComponent :type "PrimitiveComponent Object Reference"))
  (bind _asbp_player_character (cast `/Game/FirstProject/Core/Character/BP_PlayerCharacter` (`GameplayStatics.GetPlayerCharacter` 0))
    (:`then`
      (set `PlayerCharacter.itemUnderMouse` null _asbp_player_character))
    (:`CastFailed`
      (`KismetSystemLibrary.PrintString` "Emulator: Cast to Player Controller failed" true true (struct :`R` 1.0 :`A` 1.0) 5.0))))

(fn `UserConstructionScript`
  (`parent.UserConstructionScript`))